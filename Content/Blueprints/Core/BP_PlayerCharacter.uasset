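; BP_PlayerCharacter is the player character Blueprint, linking PaperZD 2D animation to the character's hit and attack states.
; On BeginPlay it casts the anim instance to AnimBPZD_PlayerCharacter and binds to its hit-finished and attack-finished events.
; Hit animations play as override sequences on that anim instance.
; When a hit animation finishes the state returns to Idle, and a finished attack calls RestoreFromAttack.
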(event `self.ReceiveBeginPlay`
  ;[1 1 1] BeginPlay
  (bind _asanim_bpzd_player_character (cast `/Game/Blueprints/PlayerCharacter/Anim/AnimBPZD_PlayerCharacter` (`PaperZDAnimationComponent.AnimInstance` (`self.PaperZDAnimation`))))
  ;[1 1 1] 绑定受击动画播放完成事件
  (add `/Game/Blueprints/PlayerCharacter/Anim/AnimBPZD_PlayerCharacter.OnHitAnimationPlayFinished` _asanim_bpzd_player_character (`|CreateDelegate` :!event `OnHitAnimationPlayFinished`))
  ;[1 1 1] 绑定攻击动画播放完成事件
  (add `/Game/Blueprints/PlayerCharacter/Anim/AnimBPZD_PlayerCharacter.OnAttackAnimationPlayFinished` _asanim_bpzd_player_character (`|CreateDelegate` :!event `OnAttackAnimationPlayFinished`)))

(event `self.PlayOverrideAnim`
  (params (InAnimSquence :type "PaperZDAnimSequence Object Reference"))
  ;[1 1 1] 覆盖播放动画
  (`PaperZDAnimInstance.K2_PlayAnimationOverride` (`PaperZDAnimationComponent.AnimInstance` (`self.PaperZDAnimation`)) InAnimSquence "DefaultSlot" 1.0 0.0))

(event `self.PlayHitAnimation`
  ;[1 1 1] 播放受击动画
  (`self.PlayOverrideAnim` "/Game/Paper2D/Character/AnimSequences/Seq_Character_Hit.Seq_Character_Hit"))

(event `OnHitAnimationPlayFinished`
  ;[1 1 1] 受击动画播放完成
  (`self.SetState` "Idle"))

(event `OnAttackAnimationPlayFinished`
  ;[1 1 1] 攻击动画播放完成
  (`self.RestoreFromAttack`))

(fn `UserConstructionScript`)