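; Player attack component that resolves combo branches and 2D attack assets for the current AttackID from data tables.
; SetupCombo rebuilds ComboMap from Combo table rows matching that ID, mapping each input command to its next attack ID.
; GetAttackSequence and GetAttackSprite look up the Skill row by ID and load its PaperZD animation sequence or judge sprite from stored paths, logging a warning if the cast fails.
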(event `self.SetupCombo`
  (`BlueprintMapLibrary.Map_Clear` (`self.ComboMap`))
  (bind _outrownames (`DataTableFunctionLibrary.GetDataTableRowNames` "/Game/Table/Combo.Combo"))
  (for _array_element _outrownames
    (bind _returnvalue (`|GetDataTableRow` "/Game/Table/Combo.Combo" _array_element)
      (:`then`
        (bind (_id _command _nextid) (break `/Game/Table/Struct/TableStruct_Combo` _returnvalue))
        (if (== _id (`self.AttackID`))
          (`BlueprintMapLibrary.Map_Add` (`self.ComboMap`) _command _nextid))))))

(fn `GetAttackSequence`
  (returns (ReturnValue :type "PaperZDAnimSequence Object Reference"))
  (bind _returnvalue (`|GetDataTableRow` "/Game/Table/Skill.Skill" (`KismetStringLibrary.Conv_StringToName` (`KismetStringLibrary.Conv_IntToString` (`self.AttackID`))))
    (:`then`
      (bind (_name _sequence) (break `/Game/Table/Struct/TableStruct_Skill` _returnvalue))
      (bind _returnvalue_2 (`GlobalBlueprintFunctionLibrary.LoadAssetByClassPath` self (`KismetSystemLibrary.MakeSoftObjectPath` _sequence)))
      (bind _aspaper_zdanim_sequence (cast `PaperZDAnimSequence` _returnvalue_2)
        (:`then`
          (return _aspaper_zdanim_sequence))
        (:`CastFailed`
          (`GlobalBlueprintFunctionLibrary.LogWarning` (`KismetStringLibrary.Concat_StrStr` "GetAttackSequence Path Invalid:" (`KismetStringLibrary.Conv_NameToString` _name))))))))

(fn `GetAttackSprite`
  (returns (ReturnValue :type "PaperSprite Object Reference"))
  (bind _returnvalue (`|GetDataTableRow` "/Game/Table/Skill.Skill" (`KismetStringLibrary.Conv_StringToName` (`KismetStringLibrary.Conv_IntToString` (`self.AttackID`))))
    (:`then`
      (bind (_name _sequence _judgesprite) (break `/Game/Table/Struct/TableStruct_Skill` _returnvalue))
      (bind _returnvalue_2 (`GlobalBlueprintFunctionLibrary.LoadAssetByClassPath` self (`KismetSystemLibrary.MakeSoftObjectPath` _judgesprite)))
      (bind _aspaper_sprite (cast `PaperSprite` _returnvalue_2)
        (:`then`
          (return _aspaper_sprite))
        (:`CastFailed`
          (`GlobalBlueprintFunctionLibrary.LogWarning` (`KismetStringLibrary.Concat_StrStr` "GetAttackSprite Path Invalid:" (`KismetStringLibrary.Conv_NameToString` _name))))))))