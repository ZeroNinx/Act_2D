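; 2D side-view player character that runs, jumps and attacks using Paper2D flipbook animations.
; Input drives movement along X, jumping and a facing flag that flips the sprite by rotation.
; Unless attacking, Tick derives idle, running, jumping or falling from velocity, stores it in PlayerStateMachine and selects the matching flipbook.
; Attack locks out those updates, plays once, then returns to Idle after a flipbook-length delay.
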(event `UpdateAnimataion`
  (params (State :type "CharacterState Enum" :default "Idle"))
  (bind _paperflipbook (`self.PaperFlipbook`))
  ;[1 1 1] 更新动画
  (`PaperFlipbookComponent.SetLooping` _paperflipbook true)
  (`PaperFlipbookComponent.SetFlipbook` _paperflipbook (select `CharacterState` State :`Idle` "/Game/Paper2D/Character/PlayerCharacter.PlayerCharacter" :`Running` "/Game/Paper2D/Character/Run/Character_Run.Character_Run" :`Jumping` "/Game/Paper2D/Character/Jump/Character_Jump_Start.Character_Jump_Start" :`Falling` "/Game/Paper2D/Character/Jump/Character_Jump_Fall.Character_Jump_Fall" :!type "PaperFlipbook Object Reference")))

(event `self.ReceiveTick`
  (params (DeltaSeconds :type "Float (single-precision)"))
  ;[1 1 1] 更新角色
  (bind _returnvalue (`self.GetState`))
  (if (!= _returnvalue (enumliteral `CharacterState` "Attacking"))
    (`self.UpdateDirection`)
    (`self.UpdateState`)
    (`self.UpdateAnimataion` _returnvalue)))

(event `InputAxis|MoveRight`
  (params (AxisValue :type "Float (single-precision)"))
  ;[1 1 1] 移动
  (if (> AxisValue 0.0)
    (set `self.bFacingRight` true)
    (`self.AddMovementInput` (1.0 0.0 0.0) AxisValue :!label _label)
    (elif (< AxisValue 0.0)
      (set `self.bFacingRight` false)
      (goto _label))))

(event `UpdateState`
  ;[1 1 1] 更新状态
  (`/Engine/EditorBlueprintResources/StandardMacros.CompareFloat` (.z (`MovementComponent.Velocity` (`self.CharacterMovement`)))
    (:`>`
      (`self.SetState` "Jumping"))
    (:`==`
      (if (!= (`KismetMathLibrary.Abs` (.x (`MovementComponent.Velocity` (`self.CharacterMovement`)))) 0.0)
        (`self.SetState` "Running")
        (else
          (`self.SetState` "Idle"))))
    (:`<`
      (`self.SetState` "Falling"))))

(event `UpdateDirection`
  (bind _paperflipbook (`self.PaperFlipbook`))
  ;[1 1 1] 调整方向
  (if (`self.bFacingRight`)
    (`SceneComponent.K2_SetWorldRotation` :`self` _paperflipbook)
    (else
      (`SceneComponent.K2_SetWorldRotation` _paperflipbook (struct :`Yaw` 180.0) false false))))

(event `InputAction|Jump`
  (params (Key :type "Key Structure"))
  ;[1 1 1] 跳跃
  (:`Pressed`
    (`self.Jump`))
  (:`Released`
    (`self.StopJumping`)))

(event `InputAction|Attack`
  (params (Key :type "Key Structure"))
  (bind _paperflipbook (`self.PaperFlipbook`))
  ;[1 1 1] 攻击
  (:`Pressed`
    (`self.SetState` "Attacking")
    (`PaperFlipbookComponent.SetFlipbook` _paperflipbook "/Game/Paper2D/Character/Attack/Attack.Attack")
    (`PaperFlipbookComponent.SetLooping` _paperflipbook false)
    (`KismetSystemLibrary.Delay` (`PaperFlipbookComponent.GetFlipbookLength` _paperflipbook))
    (`self.SetState` "Idle")
    (`PaperFlipbookComponent.SetLooping` _paperflipbook true)))

(fn `GetState`
  (returns (ReturnValue :type "CharacterState Enum"))
  (bind _returnvalue (`PlayerStateMachine.GetState` (`self.PlayerStateMachine`)))
  (return _returnvalue))

(fn `SetState`
  (params (State :type "CharacterState Enum" :default "Idle"))
  (set `PlayerStateMachine.State` State (`self.PlayerStateMachine`)))

(fn `UserConstructionScript`)