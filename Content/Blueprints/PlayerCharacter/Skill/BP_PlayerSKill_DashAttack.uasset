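; BP_PlayerSKill_DashAttack is a player skill that launches the character along the X axis and hits actors during the dash.
; When the skill judge phase begins, it picks a fixed high speed signed by the player's facing and overwrites the CharacterMovement velocity.
; Each judge tick, it queries hit actors and calls ExecuteHit on new ones, tracking them in AlreadyHitActors to prevent repeat hits.
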(event `self.OnSkillJudgeBegin`
  (`|ExecutionSequence`
    (:`then_0`
      (if (`PlayerCharacter.bFacingRight` (`GlobalBlueprintFunctionLibrary.GetPlayerCharacter`))
        (set `self.DashVelocy` 10000.0)
        (else
          (set `self.DashVelocy` -10000.0))))
    (:`then_1`
      (set `MovementComponent.Velocity` (`KismetMathLibrary.MakeVector` (`self.DashVelocy`)) (`Character.CharacterMovement` (`GlobalBlueprintFunctionLibrary.GetPlayerCharacter`))))))

(event `self.TickOnSkillJudge`
  (bind _alreadyhitactors (`self.AlreadyHitActors`))
  (bind _returnvalue (`self.GetHitActors`))
  (for _array_element _returnvalue
    (if (not (`BlueprintSetLibrary.Set_Contains` _alreadyhitactors _array_element))
      (`self.ExecuteHit` _array_element)
      (`BlueprintSetLibrary.Set_Add` _alreadyhitactors _array_element))))